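; Tower-defense turret that targets a Bug in its radius, fires bullets at it, shows a camera-facing health bar, and frees its spawn area when destroyed.
; A state variable driven on Tick switches between acquiring targets and tracking, stepping the head's yaw toward the enemy.
; Once aligned, a per-level Delay gates Dispara, which spawns a gravity-affected Bullet.
; Dispara also solves a ballistic quadratic, but the resulting pitch correction is disconnected.
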(event `self.ReceiveBeginPlay`
  ;[1 1 1] Al hacer spawn se inicializa la orientacion actual y el contador de tiempo desde el último disparo
  (set `self.state` "NewEnumerator0")
  (`self.actualizaOrientacion`)
  (`SphereComponent.SetSphereRadius` (`self.CollisionSphere`) (`self.radius`) true)
  (set `self.state` "NewEnumerator1"))

(event `self.CollisionSphere.OnComponentEndOverlap`
  (params (OverlappedComponent :type "PrimitiveComponent Object Reference") (OtherActor :type "Actor Object Reference") (OtherComp :type "PrimitiveComponent Object Reference") (OtherBodyIndex :type Integer))
  ;[1 1 1] si la torre está apuntando a un enemigo y este deja de estar en el área de acción, se vacía la variabe enemyTarget y se pasa a estado IDLE
  (if (`|EnumEquality` (`self.state`) "NewEnumerator3")
    (if (== OtherActor (`self.enemy_target`))
      (set `self.enemy_target` null)
      (set `self.state` "NewEnumerator1"))))

(event `self.ReceiveTick`
  (params (DeltaSeconds :type "Float (single-precision)"))
  (bind _towerspawnarea (`self.TowerSpawnArea`))
  (`|ExecutionSequence`
    (:`then_0`
      (if (`|EnumEquality` (`self.state`) "NewEnumerator1")
        (for _array_element (`PrimitiveComponent.GetOverlappingActors` (`self.CollisionSphere`) null)
          (`/Engine/EditorBlueprintResources/StandardMacros.IsValid` (`self.enemy_target`)
            (:`Is Valid`
              (break))
            (:`Is Not Valid`
              ;[1 1 1] Si el actor es un bicho
              (if (== (`GameplayStatics.GetObjectClass` _array_element) "/Game/TowerDefense/Blueprint/Bug.Bug_C")
                ;[1 1 1] Si la torre no ha fijado a ningún bicho, lo fija
                (set `self.enemy_target` _array_element)
                (set `self.state` "NewEnumerator3")))))))
    (:`then_1`
      ;[1 1 1] Mostrar y actualizar el porcentaje de la barra de salud
      (bind _ashud_barra_vida (cast `/Game/Maps/Interfaz/HUD_BarraVida` (`WidgetComponent.GetUserWidgetObject` (`self.BarraSalud`))))
      (`ProgressBar.SetPercent` (`/Game/Maps/Interfaz/HUD_BarraVida.ProgressBar_193` _ashud_barra_vida) (/ (`self.currentHealth`) (`self.MaxHealth`)))
      ;[1 1 1] Rotar la barra de salud hacia la cámara
      (`SceneComponent.K2_SetWorldRotation` (`self.BarraSalud`) (`KismetMathLibrary.FindLookAtRotation` (`SceneComponent.K2_GetComponentLocation` (`self.BarraSalud`)) (`PlayerController.GetFocalLocation` (`GameplayStatics.GetPlayerController` 0))) false false))
    (:`then_2`
      ;[1 1 1] Comprueba si ha muerto y se destruye
      (bind _dead (`self.Dead`))
      (if _dead
        (set `self.state` "NewEnumerator5")
        (`self.K2_DestroyActor`)
        ;[1 1 1] Permite construir de nuevo en el spawn
        (set `/Game/TowerDefense/Blueprint/TowerSpawn.CanSpawnTower` true _towerspawnarea)
        (`self.SetActorHiddenInGame` _towerspawnarea false)
        (else
          ;[1 1 1] Si la torre se encuentra en estado ORIENTING_SHOOTING, se rota la torre en la dirección del objetivo y, si está a tiro, se dispara al objetivo
          (if (`|EnumEquality` (`self.state`) "NewEnumerator3")
            (`/Engine/EditorBlueprintResources/StandardMacros.IsValid` (`self.enemy_target`) ; Si hay enemigo fijado
              (:`Is Valid`
                (bind _atiro (`self.rotaCabeza` (`self.Head`) (`self.enemy_target`) (`self.currentOrientation`)))
                (if _atiro
                  (`KismetSystemLibrary.Delay` (`|GetArrayItem` (`self.fireRate`) (`self.level`)))
                  (bind _asbug (cast `/Game/TowerDefense/Blueprint/Bug` (`self.enemy_target`)))
                  (`self.Dispara` (`SceneComponent.K2_GetComponentLocation` (`self.Cannon`)) (`SceneComponent.K2_GetComponentRotation` (`self.Head`)) _asbug))))))))))

(fn `actualizaOrientacion`
  ;[1 1 1] Se obtiene la orientación inicial de la torre a partir del vector unitario del centro de la cabeza al centro del cañón
  (set `self.currentOrientation` (`KismetMathLibrary.GetDirectionUnitVector` (`SceneComponent.K2_GetComponentLocation` (`self.Head`)) (`SceneComponent.K2_GetComponentLocation` (`self.Cannon`)))))

(fn `calculaAnguloRotacion`
  (params (head :type "SceneComponent Object Reference") (enemyTarget :type "Actor Object Reference") (currentOrientation :type "Vector Structure"))
  (returns (angulo :type "Float (double-precision)"))
  (bind _returnvalue (`KismetMathLibrary.GetDirectionUnitVector` (`SceneComponent.K2_GetComponentLocation` head) (`self.K2_GetActorLocation` enemyTarget)))
  (return (`KismetMathLibrary.Acos` (/ (`KismetMathLibrary.Dot_VectorVector` _returnvalue currentOrientation) (* (`KismetMathLibrary.VSize` _returnvalue) (`KismetMathLibrary.VSize` currentOrientation))))))

(fn `Dispara`
  (params (position :type "Vector Structure (by ref)") (orientation :type "Rotator Structure (by ref)") (bug :type "/Game/TowerDefense/Blueprint/Bug Object Reference"))
  (locals (initialLocalVelocity :type "Vector Structure" :default (0.0 0.0 0.0)) (a :type "Float (double-precision)" :default 0.0) (b :type "Float (double-precision)") (c :type "Float (double-precision)") (localBug :type "/Game/TowerDefense/Blueprint/Bug Object Reference") (gravity :type "Float (double-precision)" :default 9.8))
  (bind _returnvalue (`KismetMathLibrary.VSize2D` (- (`KismetMathLibrary.MakeVector2D` (.x (`SceneComponent.K2_GetComponentLocation` (`self.Head`))) (.y (`SceneComponent.K2_GetComponentLocation` (`self.Head`)))) (`KismetMathLibrary.MakeVector2D` (.x (`self.K2_GetActorLocation` (`local.localBug`))) (.y (`self.K2_GetActorLocation` (`local.localBug`)))))))
  (`|ExecutionSequence`
    (:`then_0`
      (set `local.localBug` bug))
    (:`then_1`
      (bind _returnvalue_2 (`|SpawnActorFromClass` "/Game/TowerDefense/Blueprint/bullet.bullet_C" (`KismetMathLibrary.MakeTransform` position orientation) "Undefined" "OverrideRootScale" null null))
      (set `/Game/TowerDefense/Blueprint/bullet.damage` (`self.Damage`) _returnvalue_2)
      (bind _projectilemovement (`/Game/TowerDefense/Blueprint/bullet.ProjectileMovement` _returnvalue_2))
      (set `ProjectileMovementComponent.ProjectileGravityScale` (`local.gravity`) _projectilemovement)
      (bind _output_get (set `local.a` (* (/ (* (`local.gravity`) (`KismetMathLibrary.Square` _returnvalue)) (* (`KismetMathLibrary.Square` (`ProjectileMovementComponent.InitialSpeed` _projectilemovement)) 2.0)) -1.0))))
    (:`then_2`
      (bind _output_get_2 (set `local.b` _returnvalue)))
    (:`then_3`
      (bind _output_get_3 (set `local.c` (+ (.z (`SceneComponent.K2_GetComponentLocation` (`self.Head`))) (`local.a`)))))
    (:`then_4`
      (bind (_resmas _resmernos) (`self.ecuacionSegundoGrado` (`local.a`) (`local.b`) (`local.c`))))))

(fn `ecuacionSegundoGrado`
  (params (a :type "Float (double-precision)") (b :type "Float (double-precision)") (c :type "Float (double-precision)"))
  (returns (resMas :type "Float (double-precision)") (resMernos :type "Float (double-precision)"))
  (locals (localA :type "Float (double-precision)") (localB :type "Float (double-precision)") (localC :type "Float (double-precision)"))
  (bind _returnvalue (* 2.0 (`local.localA`)))
  (bind _returnvalue_2 (* (`local.localB`) -1.0))
  (bind _returnvalue_3 (`KismetMathLibrary.Sqrt` (- (`KismetMathLibrary.Square` (`local.localB`)) (* 4.0 (`local.localA`) (`local.localC`)))))
  (set `local.localA` a)
  (set `local.localB` b)
  (set `local.localC` c)
  (return (/ (+ _returnvalue_2 _returnvalue_3) _returnvalue) (/ (- _returnvalue_2 _returnvalue_3) _returnvalue)))

(fn `rotaCabeza`
  (params (head :type "SceneComponent Object Reference (by ref)") (enemy :type "Actor Object Reference (by ref)") (currentOrientation :type "Vector Structure (by ref)"))
  (returns (aTiro :type Boolean))
  (bind _rotationspeed (`self.rotationSpeed`))
  (bind _returnvalue (`KismetMathLibrary.FindLookAtRotation` (`SceneComponent.K2_GetComponentLocation` head) (`self.K2_GetActorLocation` enemy)))
  (bind _yaw (.yaw (`SceneComponent.K2_GetComponentRotation` head)))
  (bind _yaw_2 (.yaw _returnvalue))
  (bind _returnvalue_2 (`KismetMathLibrary.NearlyEqual_FloatFloat` _yaw_2 _yaw 5.0))
  (if _returnvalue_2
    ;[1 1 1] si la diferencia entre ambas rotaciones es muy baja, se fija directamente la rotación (da un resultado más fluido)
    (`SceneComponent.K2_SetWorldRotation` (`self.Head`) (`KismetMathLibrary.MakeRotator` 0.0 0.0 (.yaw _returnvalue)) false false)
    (else
      ;[1 1 1] si la diferencia entre ambas rotaciones es muy alta, se desplaza la cabeza hacia esa dirección con una velocidad fija
      (`SceneComponent.K2_AddWorldRotation` (`self.Head`) (`KismetMathLibrary.MakeRotator` 0.0 0.0 (`KismetMathLibrary.SelectFloat` _rotationspeed (- 0.0 _rotationspeed) (> _yaw_2 _yaw))) false false)))
  (return _returnvalue_2))

(fn `UserConstructionScript`)