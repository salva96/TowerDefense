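; Base Blueprint for a tower defense entity, providing health tracking, damage and death handling.
; The construction script records the starting Health as MaxHealth, and TakeDamage subtracts damage while clamping Health at zero.
; Dead reports whether Health is depleted, and DestroyDeadItem uses that check to destroy the actor.
; Death is not checked inside TakeDamage, so removal relies on a separate call to DestroyDeadItem.
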(fn `Dead`
  (returns (Dead :type Boolean))
  (if (<= (`self.Health`) 0.0)
    (return true)
    (else
      (return false))))

(fn `DestroyDeadItem`
  (bind _dead (`self.Dead`))
  (if _dead
    (`self.K2_DestroyActor`)))

(fn `TakeDamage`
  (params (Damage :type "Float (double-precision) (by ref)"))
  (locals (CalculatedHealth :type "Float (double-precision)"))
  (bind _output_get (set `local.CalculatedHealth` (- (`self.Health`) Damage)))
  (if (< _output_get 0.0)
    (set `self.Health` 0.0)
    (else
      (set `self.Health` _output_get))))

(fn `UserConstructionScript`
  (set `self.MaxHealth` (`self.Health`)))