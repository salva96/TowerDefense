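; Tower defense bullet projectile that destroys itself after a short lifetime or shortly after striking a Bug.
; The construction script copies its InitialSpeed variable into the ProjectileMovement component.
; A six-second timer from BeginPlay and a brief delay after a CollisionSphere hit on an actor of exactly the Bug class both lead to the same destroy call.
; The file itself applies no damage.
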(event `self.ReceiveBeginPlay`
  (`KismetSystemLibrary.Delay` 6.0)
  (`self.K2_DestroyActor` :!label _label))

(event `self.collisionSphere.OnComponentHit`
  (params (HitComponent :type "PrimitiveComponent Object Reference") (OtherActor :type "Actor Object Reference") (OtherComp :type "PrimitiveComponent Object Reference") (NormalImpulse :type "Vector Structure") (Hit :type "HitResult Structure (by ref)"))
  (if (== (`GameplayStatics.GetObjectClass` OtherActor) "/Game/TowerDefense/Blueprint/Bug.Bug_C")
    (`KismetSystemLibrary.Delay` 0.2)
    (goto _label)))

(fn `UserConstructionScript`
  (set `ProjectileMovementComponent.InitialSpeed` (`self.initialSpeed`) (`self.ProjectileMovement`)))