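; Tower3 is a tower defense tower variant that extends a parent tower with its own firing gravity and targeting rule.
; Dispara calls the parent shot with a fixed Gravity, overriding the incoming value.
; FijaObjetivo scans Bugs overlapping CollisionSphere, favoring highest MaxHealth, then shortest distance.
; As wired, only that distance tie-break assigns EnemyTarget and it zeroes DistanciaMin; any valid target switches the tower's State.
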(event `self.ReceiveTick`
  (params (DeltaSeconds :type "Float (single-precision)"))
  (`parent.ReceiveTick` DeltaSeconds))

(fn `Dispara`
  (params (position :type "Vector Structure (by ref)") (orientation :type "Rotator Structure (by ref)") (bug :type "/Game/TowerDefense/Blueprint/Bug Object Reference") (gravity :type "Float (double-precision)"))
  (`parent.Dispara` position orientation bug 4.5)
  (return))

(fn `fijaObjetivo`
  (locals (enemigoAct :type "Actor Object Reference") (distanciaMin :type "Float (double-precision)") (vidaMax :type "Float (double-precision)"))
  (bind _vidamax (`local.vidaMax`))
  (for _array_element (`PrimitiveComponent.GetOverlappingActors` (`self.CollisionSphere`) null)
    ;[1 1 1] Si el actor es un bicho
    (if (`KismetMathLibrary.ClassIsChildOf` (`GameplayStatics.GetObjectClass` _array_element) "/Game/TowerDefense/Blueprint/Bug.Bug_C")
      (bind _output_get (set `local.enemigoAct` _array_element))
      ;[1 1 1] se comprueba si la vida máxima de este enemigo es mayor o igual que la vida máxima actual
      (bind _asbug (cast `/Game/TowerDefense/Blueprint/Bug` _output_get))
      (bind _maxhealth (`/Game/TowerDefense/Blueprint/TowerDefenseEntity.MaxHealth` _asbug))
      ;[1 1 1] si tiene mayor vida máxima, se actualiza la vida máxima y la distancia mínima y se fija el enemyTarget
      (if (> _maxhealth _vidamax)
        (set `local.vidaMax` _maxhealth)
        (set `local.distanciaMin` (`KismetMathLibrary.VSize` (- (`self.K2_GetActorLocation`) (`self.K2_GetActorLocation`))))
        (else
          ;[1 1 1] si tiene la mimsa vida, se comprueba si la distancia a este enemigo es la menor hasta ahora, en caso afirmativo, se fija a este enemigo como enemyTarget
          (if (== _maxhealth _vidamax)
            (if (< (`KismetMathLibrary.VSize` (- (`self.K2_GetActorLocation`) (`self.K2_GetActorLocation`))) (`local.distanciaMin`))
              (set `local.distanciaMin` 0.0)
              (set `self.enemy_target` (`local.enemigoAct`))))))))
  ;[1 1 1] i se ha fijado objetivo, se pasa al estado orienting_shooting
  (`/Engine/EditorBlueprintResources/StandardMacros.IsValid` (`self.enemy_target`)
    (:`Is Valid`
      (set `self.state` "NewEnumerator3"))))

(fn `UserConstructionScript`
  (`parent.UserConstructionScript`))