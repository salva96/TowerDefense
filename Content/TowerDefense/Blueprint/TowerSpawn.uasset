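; TowerSpawn is a clickable tower defense tile that opens the tower selection menu when a tower can be placed on it.
; Mouse hover, click and release events on its StaticMesh swap materials as feedback, turning it red when CanSpawnTower is false.
; An allowed click removes any open HUD_SelectorTorre widgets, then creates a new one and passes this tile as its TowerArea.
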(event `self.StaticMesh.OnBeginCursorOver`
  (params (TouchedComponent :type "PrimitiveComponent Object Reference"))
  (`KismetSystemLibrary.PrintString` "CURSOR ENCIMA")
  (`PrimitiveComponent.SetMaterial` (`self.StaticMesh`) 0 "/Game/Terreno/Materials/color_verde.color_verde"))

(event `self.StaticMesh.OnEndCursorOver`
  (params (TouchedComponent :type "PrimitiveComponent Object Reference"))
  (`PrimitiveComponent.SetMaterial` (`self.StaticMesh`) 0 "/Engine/VREditor/LaserPointer/HoverMaterial.HoverMaterial"))

(event `self.StaticMesh.OnClicked`
  (params (TouchedComponent :type "PrimitiveComponent Object Reference") (ButtonPressed :type "Key Structure"))
  (bind _staticmesh (`self.StaticMesh`))
  (`KismetSystemLibrary.PrintString` "asssssssssssssssssssssssssssssssssssssssssssss")
  (if (`self.CanSpawnTower`)
    (`PrimitiveComponent.SetMaterial` _staticmesh 0 "/Game/Terreno/Materials/color_verde.color_verde")
    ;[1 1 1] Quitar el menú de selección de torre del HUD si estaba abierto por otra casilla y abrir el menú en esta casilla
    (bind _foundwidgets (`WidgetBlueprintLibrary.GetAllWidgetsOfClass` "/Game/Maps/Interfaz/HUD_SelectorTorre.HUD_SelectorTorre_C" false))
    (for _array_element _foundwidgets
      (`Widget.RemoveFromParent` _array_element))
    (bind _returnvalue (`|CreateWidget` "/Game/Maps/Interfaz/HUD_SelectorTorre.HUD_SelectorTorre_C"))
    (`UserWidget.AddToViewport` _returnvalue 0)
    (set `/Game/Maps/Interfaz/HUD_SelectorTorre.TowerArea` self _returnvalue)
    (else
      (`PrimitiveComponent.SetMaterial` _staticmesh 0 "/Game/Terreno/Materials/color_rojo.color_rojo"))))

(event `self.StaticMesh.OnReleased`
  (params (TouchedComponent :type "PrimitiveComponent Object Reference") (ButtonReleased :type "Key Structure"))
  (`PrimitiveComponent.SetMaterial` (`self.StaticMesh`) 0 "/Game/Terreno/Materials/color_naranja.color_naranja"))

(fn `UserConstructionScript`)