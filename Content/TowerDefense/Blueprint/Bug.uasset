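; Spider enemy for a tower defense game that walks along a Path spline, attacks blockers and awards energy on death.
; Tick drives an animation state machine and turns the health bar toward the camera.
; CanMove projects a probe box to the next spline distance to test TowerDefenseEntity overlaps: bugs wait behind other bugs or at path end, and damage other entities.
; Bullets overlapping its Box damage it.
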(event `self.ReceiveTick`
  (params (DeltaSeconds :type "Float (single-precision)"))
  ;[1 1 1] Mostrar y actualizar el porcentaje de la barra de salud
  (bind _ashud_barra_vida (cast `/Game/Maps/Interfaz/HUD_BarraVida` (`WidgetComponent.GetUserWidgetObject` (`self.BarraSalud`))))
  (`ProgressBar.SetPercent` (`/Game/Maps/Interfaz/HUD_BarraVida.ProgressBar_193` _ashud_barra_vida) (/ (`self.Health`) (`self.MaxHealth`)))
  ;[1 1 1] Rotar la barra de salud hacia la cámara
  (`SceneComponent.K2_SetWorldRotation` (`self.BarraSalud`) (`KismetMathLibrary.FindLookAtRotation` (`SceneComponent.K2_GetComponentLocation` (`self.BarraSalud`)) (`PlayerController.GetFocalLocation` (`GameplayStatics.GetPlayerController` 0))) false false)
  (`/Engine/EditorBlueprintResources/StandardMacros.IsValid` (`self.Path`)
    (:`Is Valid`
      (bind _dead (`self.Dead`))
      (if _dead
        (if (`|EnumInequality` (`self.State`) "NewEnumerator3")
          (set `self.State` "NewEnumerator3")
          (`SkeletalMeshComponent.PlayAnimation` (`self.Mesh`) "/Game/Spider/Spider_3_Anim_Spider_Armature_die.Spider_3_Anim_Spider_Armature_die" false)
          (`KismetSystemLibrary.Delay` (`self.DyingLapse`))
          (bind _asmy_game_instance (cast `/Game/MyGameInstance` (`GameplayStatics.GetGameInstance`)))
          (set `/Game/MyGameInstance.currentEnergy` (+ (`/Game/MyGameInstance.currentEnergy` _asmy_game_instance) (`self.energy`)) _asmy_game_instance)
          (`self.K2_DestroyActor`))
        (elif (`|EnumInequality` (`self.State`) "NewEnumerator1")
          (bind (_canmove _distance _collisionwith) (`self.CanMove`))
          (if _canmove
            (if (`|EnumInequality` (`self.State`) "NewEnumerator2")
              (set `self.State` "NewEnumerator2")
              (`SkeletalMeshComponent.PlayAnimation` (`self.Mesh`) "/Game/Spider/Spider_3_Anim_Spider_Armature_run_ani_vor.Spider_3_Anim_Spider_Armature_run_ani_vor" true))
            (set `self.DistanceAlongPath` _distance)
            (`self.UpdateLocationAndRotation`)
            (elif (`KismetSystemLibrary.IsValid` _collisionwith)
              (if (== (`GameplayStatics.GetObjectClass` _collisionwith) "Bug_C")
                (if (`|EnumInequality` (`self.State`) "NewEnumerator0") :!label _label
                  (set `self.State` "NewEnumerator0")
                  (`SkeletalMeshComponent.PlayAnimation` (`self.Mesh`) null true))
                (elif (`|EnumInequality` (`self.State`) "NewEnumerator1")
                  (set `self.State` "NewEnumerator1")
                  (`self.K2_SetActorRotation` (`KismetMathLibrary.FindLookAtRotation` (`self.K2_GetActorLocation`) (`self.K2_GetActorLocation` _collisionwith)))
                  (`SkeletalMeshComponent.PlayAnimation` (`self.Mesh`) "/Game/Spider/Spider_3_Anim_Spider_Armature_Attack.Spider_3_Anim_Spider_Armature_Attack" false)
                  (`KismetSystemLibrary.PrintString` (`KismetSystemLibrary.GetDisplayName` _collisionwith))
                  (`self.TakeDamage` _collisionwith (`self.Damage`))
                  (`KismetSystemLibrary.Delay` 1.5)
                  (set `self.State` "NewEnumerator0")
                  (`SkeletalMeshComponent.PlayAnimation` (`self.Mesh`) "/Game/Spider/Spider_3_Anim_Spider_Armature_normal.Spider_3_Anim_Spider_Armature_normal" true)))
              (else
                (goto _label)))))))))

(event `self.Box.OnComponentBeginOverlap`
  (params (OverlappedComponent :type "PrimitiveComponent Object Reference") (OtherActor :type "Actor Object Reference") (OtherComp :type "PrimitiveComponent Object Reference") (OtherBodyIndex :type Integer) (bFromSweep :type Boolean) (SweepResult :type "HitResult Structure (by ref)"))
  (if (== (`GameplayStatics.GetObjectClass` OtherActor) "/Game/TowerDefense/Blueprint/bullet.bullet_C")
    (bind _asbullet (cast `/Game/TowerDefense/Blueprint/bullet` OtherActor))
    (`self.TakeDamage` (`/Game/TowerDefense/Blueprint/bullet.damage` _asbullet))))

(fn `CanMove`
  (returns (CanMove :type Boolean) (Distance :type "Float (double-precision)") (CollisionWith :type "/Game/TowerDefense/Blueprint/TowerDefenseEntity Object Reference"))
  (locals (Allowed :type Boolean :default true) (OriginalBoxMovementTransform :type "Transform Structure") (NextDis :type "Float (double-precision)") (Collision :type "/Game/TowerDefense/Blueprint/TowerDefenseEntity Object Reference"))
  (bind (_originalboxmovementtransform_location _originalboxmovementtransform_rotation _originalboxmovementtransform_scale) (`KismetMathLibrary.BreakTransform` (`local.OriginalBoxMovementTransform`)))
  (bind _distance (`self.NextDistance`))
  (bind _output_get (set `local.NextDis` _distance))
  (bind _end (`self.OutOfPath` _output_get))
  (if _end
    (return false _output_get null)
    (else
      (set `local.OriginalBoxMovementTransform` (`SceneComponent.GetRelativeTransform` (`self.BoxMovement`)))
      (bind _transform (`self.TransformOfDistance` (`local.NextDis`)))
      (`SceneComponent.K2_SetWorldTransform` (`self.BoxMovement`) (`KismetMathLibrary.MakeTransform` (+ (.location _transform) _originalboxmovementtransform_location) (`KismetMathLibrary.ComposeRotators` _originalboxmovementtransform_rotation (.rotation _transform)) _originalboxmovementtransform_scale) false false)
      (bind _outactors (`GameplayStatics.GetAllActorsOfClass` "/Game/TowerDefense/Blueprint/TowerDefenseEntity.TowerDefenseEntity_C"))
      (for _array_element _outactors
        (bind _box (`/Game/TowerDefense/Blueprint/TowerDefenseEntity.Box` _array_element))
        (if (!= (`self.Box`) _box)
          (bind _overlapping (`/Game/TowerDefense/Blueprint/TowerDefense.IsOverlappingCollisionBox` (`self.BoxMovement`) _box))
          (if _overlapping
            (set `local.Collision` _array_element)
            (set `local.Allowed` false)
            (break))))
      (`SceneComponent.K2_SetRelativeTransform` (`self.BoxMovement`) (`local.OriginalBoxMovementTransform`) false false)
      (return (`local.Allowed`) (`local.NextDis`) (`local.Collision`)))))

(fn `NextDistance`
  (returns (Distance :type "Float (double-precision)"))
  (return (+ (`self.DistanceAlongPath`) (* (`GameplayStatics.GetWorldDeltaSeconds`) (`self.BugSpeed`)))))

(fn `OutOfPath`
  (params (Distance :type "Float (double-precision) (by ref)"))
  (returns (End :type Boolean))
  (if (> Distance (`SplineComponent.GetSplineLength` (`/Game/TowerDefense/Blueprint/SplineShape.Spline` (`self.Path`))))
    (return true)
    (else
      (return false))))

(fn `TransformOfDistance`
  (params (Distance :type "Float (double-precision) (by ref)"))
  (returns (Transform :type "Transform Structure"))
  (bind _spline (`/Game/TowerDefense/Blueprint/SplineShape.Spline` (`self.Path`)))
  (return (`KismetMathLibrary.MakeTransform` (`SplineComponent.GetLocationAtDistanceAlongSpline` _spline Distance "World") (`SplineComponent.GetRotationAtDistanceAlongSpline` _spline Distance "World"))))

(fn `UpdateLocationAndRotation`
  (bind _transform (`self.TransformOfDistance` (`self.DistanceAlongPath`)))
  (`self.K2_SetActorLocationAndRotation` (.location _transform) (.rotation _transform)))

(fn `UserConstructionScript`)