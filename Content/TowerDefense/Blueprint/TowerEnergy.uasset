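; TowerEnergy is a tower defense tower actor that displays its health and frees its build spot when it dies.
; Each Tick it writes the health ratio to its HUD_BarraVida widget's progress bar and rotates that bar toward the player controller's focal location.
; The same Tick checks Dead(), then destroys the actor and makes its TowerSpawnArea visible and available for building again.
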(event `self.ReceiveTick`
  (params (DeltaSeconds :type "Float (single-precision)"))
  (bind _towerspawnarea (`self.TowerSpawnArea`))
  ;[1 1 1] Mostrar y actualizar el porcentaje de la barra de salud
  (bind _ashud_barra_vida (cast `/Game/Maps/Interfaz/HUD_BarraVida` (`WidgetComponent.GetUserWidgetObject` (`self.BarraSalud`))))
  (`ProgressBar.SetPercent` (`/Game/Maps/Interfaz/HUD_BarraVida.ProgressBar_193` _ashud_barra_vida) (/ (`self.Health`) (`self.MaxHealth`)))
  ;[1 1 1] Rotar la barra de salud hacia la cámara
  (`SceneComponent.K2_SetWorldRotation` (`self.BarraSalud`) (`KismetMathLibrary.FindLookAtRotation` (`SceneComponent.K2_GetComponentLocation` (`self.BarraSalud`)) (`PlayerController.GetFocalLocation` (`GameplayStatics.GetPlayerController` 0))) false false)
  ;[1 1 1] Comprueba si ha muerto y se destruye
  (bind _dead (`self.Dead`))
  (if _dead
    (`self.K2_DestroyActor`)
    ;[1 1 1] Permite construir de nuevo
    (set `/Game/TowerDefense/Blueprint/TowerSpawn.CanSpawnTower` true _towerspawnarea)
    (`self.SetActorHiddenInGame` _towerspawnarea false)))

(fn `UserConstructionScript`)