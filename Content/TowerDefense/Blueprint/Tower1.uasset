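; Tower1 is a tower-defense tower Blueprint that inherits its tick, construction and firing behavior from a parent class.
; It overrides the pseudo-parabolic shot only to call the parent with a fixed gravity value.
; Its targeting function scans Bug actors overlapping the collision sphere, keeps the one closer than the stored minimum distance, and switches to the orienting-and-shooting state when a target is valid.
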(event `self.ReceiveTick`
  (params (DeltaSeconds :type "Float (single-precision)"))
  (`parent.ReceiveTick` DeltaSeconds))

(fn `Dispara Pseudoparabólico`
  (params (position :type "Vector Structure (by ref)") (orientation :type "Rotator Structure (by ref)") (bug :type "/Game/TowerDefense/Blueprint/Bug Object Reference") (gravity :type "Float (double-precision)"))
  (`parent.Dispara Pseudoparabólico` position orientation bug 7.0)
  (return))

(fn `fijaObjetivo`
  (locals (distanciaMin :type "Float (double-precision)" :default 10000000.0) (enemigoAct :type "Actor Object Reference"))
  (bind _returnvalue (`KismetMathLibrary.VSize` (- (`self.K2_GetActorLocation` (`local.enemigoAct`)) (`self.K2_GetActorLocation`))))
  (for _array_element (`PrimitiveComponent.GetOverlappingActors` (`self.CollisionSphere`) null)
    ;[1 1 1] Si el actor es un bicho
    (if (`KismetMathLibrary.ClassIsChildOf` (`GameplayStatics.GetObjectClass` _array_element) "/Game/TowerDefense/Blueprint/Bug.Bug_C")
      (set `local.enemigoAct` _array_element)
      ;[1 1 1] si la distancia a este enemigo es la menor hasta ahora, se fija a este enemigo
      (if (< _returnvalue (`local.distanciaMin`))
        (set `local.distanciaMin` _returnvalue)
        (set `self.enemy_target` (`local.enemigoAct`)))))
  ;[1 1 1] Si se ha fijado objetivo, se pasa al estado orienting_shooting
  (`/Engine/EditorBlueprintResources/StandardMacros.IsValid` (`self.enemy_target`)
    (:`Is Valid`
      (set `self.state` "NewEnumerator3"))))

(fn `UserConstructionScript`
  (`parent.UserConstructionScript`))