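; Tower defense bug spawner that produces a set number of bugs, then bosses, along an assigned spline Path, destroying itself if none is set.
; Start and Stop control it; Tick launches a delayed loop that spawns only when no bug overlaps its box.
; CreateBug picks one of three types at random, enlarging and strengthening bosses.
; The boss loop has no delay and ends when the box is blocked.
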(event `self.ReceiveTick`
  (params (DeltaSeconds :type "Float (single-precision)"))
  (if (not (`self.Started`))
    (set `self.Started` true)
    (if (`self.Active`) :!label _label
      (if (> (`self.Bugs`) 0)
        (bind _free (`self.IsSpawnFree`))
        (if _free
          (`self.CreateBug` false)
          (set `self.Bugs` (- (`self.Bugs`) 1)))
        (`KismetSystemLibrary.Delay` (`self.Delay`))
        (goto _label)
        (else
          (if (> (`self.Bosses`) 0) :!label _label_2
            (bind _free_2 (`self.IsSpawnFree`))
            (if _free_2
              (set `self.Bosses` (- (`self.Bosses`) 1))
              (`self.CreateBug` true)
              (goto _label_2))
            (else
              (set `self.Active` false))))))))

(event `self.ReceiveBeginPlay`
  (if (not (`KismetSystemLibrary.IsValid` (`self.Path`)))
    (`self.K2_DestroyActor`)))

(fn `CreateBug`
  (params (IsBoss :type Boolean :default false))
  (locals (IsBoss2 :type Boolean) (Bug :type "/Game/TowerDefense/Blueprint/Bug Object Reference"))
  (bind _bug (`local.Bug`))
  (bind _returnvalue (`KismetMathLibrary.MakeTransform` (`SceneComponent.K2_GetComponentLocation` (`self.DefaultSceneRoot`)) (`SplineComponent.GetRotationAtDistanceAlongSpline` (`/Game/TowerDefense/Blueprint/SplineShape.Spline` (`self.Path`)) 0.0 "World")))
  (set `local.IsBoss2` IsBoss)
  (switch `int` (`KismetMathLibrary.RandomInteger` 3)
    (:`0`
      (bind _returnvalue_2 (`|SpawnActorFromClass` "/Game/TowerDefense/Blueprint/BugType1.BugType1_C" _returnvalue "AlwaysSpawn" "OverrideRootScale" null null))
      (set `local.Bug` _returnvalue_2))
    (:`1`
      (bind _returnvalue_3 (`|SpawnActorFromClass` "/Game/TowerDefense/Blueprint/BugType2.BugType2_C" _returnvalue "AlwaysSpawn" "OverrideRootScale" null null))
      (set `local.Bug` _returnvalue_3))
    (:`2`
      (bind _returnvalue_4 (`|SpawnActorFromClass` "/Game/TowerDefense/Blueprint/BugType3.BugType3_C" _returnvalue "AlwaysSpawn" "OverrideRootScale" null null))
      (set `local.Bug` _returnvalue_4)))
  (if (`local.IsBoss2`)
    (`self.SetBossProperties` _bug))
  (set `/Game/TowerDefense/Blueprint/Bug.Path` (`self.Path`) _bug))

(fn `IsSpawnFree`
  (returns (Free :type Boolean))
  (bind _outactors (`GameplayStatics.GetAllActorsOfClass` "/Game/TowerDefense/Blueprint/Bug.Bug_C"))
  (for _array_element _outactors
    (bind _overlapping (`/Game/TowerDefense/Blueprint/TowerDefense.IsOverlappingCollisionBox` (`self.Box`) (`/Game/TowerDefense/Blueprint/TowerDefenseEntity.Box` _array_element)))
    (if _overlapping
      (return false)))
  (return true))

(fn `SetBossProperties`
  (params (BugBoss :type "/Game/TowerDefense/Blueprint/Bug Object Reference (by ref)"))
  (`self.SetActorScale3D` BugBoss (5.0 5.0 5.0))
  (set `/Game/TowerDefense/Blueprint/TowerDefenseEntity.Damage` 30.0 BugBoss)
  (set `/Game/TowerDefense/Blueprint/TowerDefenseEntity.Health` 300.0 BugBoss)
  (set `/Game/TowerDefense/Blueprint/Bug.energy` 100 BugBoss))

(fn `Start`
  (params (NumBugs :type "Integer (by ref)") (NumBosses :type "Integer (by ref)"))
  ;[1 1 1] Inicia el Bug Spawner para que fabrique la cantidad de bichos indicada.
  (set `self.Bugs` NumBugs)
  (set `self.Bosses` NumBosses)
  (set `self.Active` true)
  (set `self.Started` false))

(fn `Stop`
  ;[1 1 1] Para el Bug Spawner para que no produzca más bichos.
  (set `self.Active` false))

(fn `UserConstructionScript`
  (if (`self.Active`)
    (set `self.Started` false)
    (else
      (set `self.Started` true))))