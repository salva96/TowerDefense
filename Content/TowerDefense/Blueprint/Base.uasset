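; Base Blueprint for a tower defense game object with health, displayed on a BarraSalud widget health bar.
; Each Tick sets the HUD_BarraVida progress bar from current over max health and turns the bar toward the player controller's focal location.
; It then calls DestroyDeadItem, whose body is not in this graph, to check for death and destroy the object.
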(event `self.ReceiveTick`
  (params (DeltaSeconds :type "Float (single-precision)"))
  ;[1 1 1] Mostrar y actualizar el porcentaje de la barra de salud
  (bind _ashud_barra_vida (cast `/Game/Maps/Interfaz/HUD_BarraVida` (`WidgetComponent.GetUserWidgetObject` (`self.BarraSalud`))))
  (`ProgressBar.SetPercent` (`/Game/Maps/Interfaz/HUD_BarraVida.ProgressBar_193` _ashud_barra_vida) (/ (`self.currentHealth`) (`self.MaxHealth`)))
  ;[1 1 1] Rotar la barra de salud hacia la cámara
  (`SceneComponent.K2_SetWorldRotation` (`self.BarraSalud`) (`KismetMathLibrary.FindLookAtRotation` (`SceneComponent.K2_GetComponentLocation` (`self.BarraSalud`)) (`PlayerController.GetFocalLocation` (`GameplayStatics.GetPlayerController` 0))) false false)
  ;[1 1 1] Comprueba si ha muerto y se destruye
  (`self.DestroyDeadItem`))

(fn `UserConstructionScript`)